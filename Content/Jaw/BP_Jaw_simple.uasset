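; Jaw model Blueprint that gives its static mesh parts mouse-over highlighting through material parameters.
; Most meshes toggle a "selected" scalar on cursor enter and exit, while StaticMesh15 to 18 switch their "color" vector between red and grey.
; StaticMesh14 instead drives StaticMesh15, stepping it through green, yellow and red with delays; leaving restores grey but does not cancel pending steps.
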(event `self.StaticMesh1.OnBeginCursorOver`
  (params (TouchedComponent :type "PrimitiveComponent Object Reference"))
  (`MeshComponent.SetScalarParameterValueOnMaterials` (`self.StaticMesh1`) "selected" 1.0))

(event `self.StaticMesh1.OnEndCursorOver`
  (params (TouchedComponent :type "PrimitiveComponent Object Reference"))
  (`MeshComponent.SetScalarParameterValueOnMaterials` (`self.StaticMesh1`) "selected" 0.0))

(event `self.StaticMesh2.OnBeginCursorOver`
  (params (TouchedComponent :type "PrimitiveComponent Object Reference"))
  (`MeshComponent.SetScalarParameterValueOnMaterials` (`self.StaticMesh2`) "selected" 1.0))

(event `self.StaticMesh2.OnEndCursorOver`
  (params (TouchedComponent :type "PrimitiveComponent Object Reference"))
  (`MeshComponent.SetScalarParameterValueOnMaterials` (`self.StaticMesh2`) "selected" 0.0))

(event `self.StaticMesh4.OnBeginCursorOver`
  (params (TouchedComponent :type "PrimitiveComponent Object Reference"))
  (`MeshComponent.SetScalarParameterValueOnMaterials` (`self.StaticMesh4`) "selected" 1.0))

(event `self.StaticMesh4.OnEndCursorOver`
  (params (TouchedComponent :type "PrimitiveComponent Object Reference"))
  (`MeshComponent.SetScalarParameterValueOnMaterials` (`self.StaticMesh4`) "selected" 0.0))

(event `self.StaticMesh3.OnBeginCursorOver`
  (params (TouchedComponent :type "PrimitiveComponent Object Reference"))
  (`MeshComponent.SetScalarParameterValueOnMaterials` (`self.StaticMesh3`) "selected" 1.0))

(event `self.StaticMesh3.OnEndCursorOver`
  (params (TouchedComponent :type "PrimitiveComponent Object Reference"))
  (`MeshComponent.SetScalarParameterValueOnMaterials` (`self.StaticMesh3`) "selected" 0.0))

(event `self.StaticMesh5.OnBeginCursorOver`
  (params (TouchedComponent :type "PrimitiveComponent Object Reference"))
  (`MeshComponent.SetScalarParameterValueOnMaterials` (`self.StaticMesh5`) "selected" 1.0))

(event `self.StaticMesh5.OnEndCursorOver`
  (params (TouchedComponent :type "PrimitiveComponent Object Reference"))
  (`MeshComponent.SetScalarParameterValueOnMaterials` (`self.StaticMesh5`) "selected" 0.0))

(event `self.StaticMesh6.OnBeginCursorOver`
  (params (TouchedComponent :type "PrimitiveComponent Object Reference"))
  (`MeshComponent.SetScalarParameterValueOnMaterials` (`self.StaticMesh6`) "selected" 1.0))

(event `self.StaticMesh6.OnEndCursorOver`
  (params (TouchedComponent :type "PrimitiveComponent Object Reference"))
  (`MeshComponent.SetScalarParameterValueOnMaterials` (`self.StaticMesh6`) "selected" 0.0))

(event `self.StaticMesh7.OnBeginCursorOver`
  (params (TouchedComponent :type "PrimitiveComponent Object Reference"))
  (`MeshComponent.SetScalarParameterValueOnMaterials` (`self.StaticMesh7`) "selected" 1.0))

(event `self.StaticMesh7.OnEndCursorOver`
  (params (TouchedComponent :type "PrimitiveComponent Object Reference"))
  (`MeshComponent.SetScalarParameterValueOnMaterials` (`self.StaticMesh7`) "selected" 0.0))

(event `self.StaticMesh8.OnBeginCursorOver`
  (params (TouchedComponent :type "PrimitiveComponent Object Reference"))
  (`MeshComponent.SetScalarParameterValueOnMaterials` (`self.StaticMesh8`) "selected" 1.0))

(event `self.StaticMesh8.OnEndCursorOver`
  (params (TouchedComponent :type "PrimitiveComponent Object Reference"))
  (`MeshComponent.SetScalarParameterValueOnMaterials` (`self.StaticMesh8`) "selected" 0.0))

(event `self.StaticMesh9.OnBeginCursorOver`
  (params (TouchedComponent :type "PrimitiveComponent Object Reference"))
  (`MeshComponent.SetScalarParameterValueOnMaterials` (`self.StaticMesh9`) "selected" 1.0))

(event `self.StaticMesh9.OnEndCursorOver`
  (params (TouchedComponent :type "PrimitiveComponent Object Reference"))
  (`MeshComponent.SetScalarParameterValueOnMaterials` (`self.StaticMesh9`) "selected" 0.0))

(event `self.StaticMesh10.OnBeginCursorOver`
  (params (TouchedComponent :type "PrimitiveComponent Object Reference"))
  (`MeshComponent.SetScalarParameterValueOnMaterials` (`self.StaticMesh10`) "selected" 1.0))

(event `self.StaticMesh10.OnEndCursorOver`
  (params (TouchedComponent :type "PrimitiveComponent Object Reference"))
  (`MeshComponent.SetScalarParameterValueOnMaterials` (`self.StaticMesh10`) "selected" 0.0))

(event `self.StaticMesh11.OnBeginCursorOver`
  (params (TouchedComponent :type "PrimitiveComponent Object Reference"))
  (`MeshComponent.SetScalarParameterValueOnMaterials` (`self.StaticMesh11`) "selected" 1.0))

(event `self.StaticMesh11.OnEndCursorOver`
  (params (TouchedComponent :type "PrimitiveComponent Object Reference"))
  (`MeshComponent.SetScalarParameterValueOnMaterials` (`self.StaticMesh11`) "selected" 0.0))

(event `self.StaticMesh12.OnBeginCursorOver`
  (params (TouchedComponent :type "PrimitiveComponent Object Reference"))
  (`MeshComponent.SetScalarParameterValueOnMaterials` (`self.StaticMesh12`) "selected" 1.0))

(event `self.StaticMesh12.OnEndCursorOver`
  (params (TouchedComponent :type "PrimitiveComponent Object Reference"))
  (`MeshComponent.SetScalarParameterValueOnMaterials` (`self.StaticMesh12`) "selected" 0.0))

(event `self.StaticMesh13.OnBeginCursorOver`
  (params (TouchedComponent :type "PrimitiveComponent Object Reference"))
  (`MeshComponent.SetScalarParameterValueOnMaterials` (`self.StaticMesh13`) "selected" 1.0))

(event `self.StaticMesh13.OnEndCursorOver`
  (params (TouchedComponent :type "PrimitiveComponent Object Reference"))
  (`MeshComponent.SetScalarParameterValueOnMaterials` (`self.StaticMesh13`) "selected" 0.0))

(event `self.StaticMesh14.OnBeginCursorOver`
  (params (TouchedComponent :type "PrimitiveComponent Object Reference"))
  (bind _staticmesh15 (`self.StaticMesh15`))
  (`MeshComponent.SetVectorParameterValueOnMaterials` _staticmesh15 "color" (0.101199 0.658333 0.160537))
  (`KismetSystemLibrary.Delay` 1.5)
  (`MeshComponent.SetVectorParameterValueOnMaterials` _staticmesh15 "color" (0.658333 0.630142 0.064095))
  (`KismetSystemLibrary.Delay` 1.5)
  (`MeshComponent.SetVectorParameterValueOnMaterials` _staticmesh15 "color" (1.0 0.0 0.0)))

(event `self.StaticMesh14.OnEndCursorOver`
  (params (TouchedComponent :type "PrimitiveComponent Object Reference"))
  (`MeshComponent.SetVectorParameterValueOnMaterials` (`self.StaticMesh15`) "color" (0.61 0.65 0.65)))

(event `self.StaticMesh15.OnBeginCursorOver`
  (params (TouchedComponent :type "PrimitiveComponent Object Reference"))
  (`MeshComponent.SetVectorParameterValueOnMaterials` (`self.StaticMesh15`) "color" (1.0 0.0 0.0)))

(event `self.StaticMesh15.OnEndCursorOver`
  (params (TouchedComponent :type "PrimitiveComponent Object Reference"))
  (`MeshComponent.SetVectorParameterValueOnMaterials` (`self.StaticMesh15`) "color" (0.611 0.65 0.65)))

(event `self.StaticMesh16.OnBeginCursorOver`
  (params (TouchedComponent :type "PrimitiveComponent Object Reference"))
  (`MeshComponent.SetVectorParameterValueOnMaterials` (`self.StaticMesh16`) "color" (1.0 0.0 0.0)))

(event `self.StaticMesh16.OnEndCursorOver`
  (params (TouchedComponent :type "PrimitiveComponent Object Reference"))
  (`MeshComponent.SetVectorParameterValueOnMaterials` (`self.StaticMesh16`) "color" (0.61 0.65 0.65)))

(event `self.StaticMesh17.OnBeginCursorOver`
  (params (TouchedComponent :type "PrimitiveComponent Object Reference"))
  (`MeshComponent.SetVectorParameterValueOnMaterials` (`self.StaticMesh17`) "color" (1.0 0.0 0.0)))

(event `self.StaticMesh17.OnEndCursorOver`
  (params (TouchedComponent :type "PrimitiveComponent Object Reference"))
  (`MeshComponent.SetVectorParameterValueOnMaterials` (`self.StaticMesh17`) "color" (0.61 0.65 0.65)))

(event `self.StaticMesh18.OnBeginCursorOver`
  (params (TouchedComponent :type "PrimitiveComponent Object Reference"))
  (`MeshComponent.SetVectorParameterValueOnMaterials` (`self.StaticMesh18`) "color" (1.0 0.0 0.0)))

(event `self.StaticMesh18.OnEndCursorOver`
  (params (TouchedComponent :type "PrimitiveComponent Object Reference"))
  (`MeshComponent.SetVectorParameterValueOnMaterials` (`self.StaticMesh18`) "color" (0.61 0.65 0.65)))

(fn `UserConstructionScript`)