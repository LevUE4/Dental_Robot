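; Lower jaw model that visualizes live tooth touch and zone force data from a remote server.
; A looping timer requests jaw data over HTTP every tenth of a second.
; When the data arrives, touch values toggle each tooth material's "selected" parameter and zone forces set it proportionally on four Force components.
; Tooth checks are partly nested, so several later teeth update only while Tooth4, Tooth5, Tooth10 or Tooth11 are touched.
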(event `self.ReceiveBeginPlay`
  (`KismetSystemLibrary.K2_SetTimerDelegate` (delegate `DataRefresh`) 0.1 true))

(event `DataRefresh`
  (`self.requestHttpJawData` "http://wan1.at.pstu.ru:8008/"))

(event `self.PullingDataComplete`
  (bind _tooth_13 (`self.Tooth_13`))
  (bind _tooth_2 (`self.Tooth_2`))
  (bind _tooth_3 (`self.Tooth_3`))
  (bind _tooth_4 (`self.Tooth_4`))
  (bind _tooth_5 (`self.Tooth_5`))
  (bind _tooth_1 (`self.Tooth_1`))
  (bind _tooth_6 (`self.Tooth_6`))
  (bind _tooth_7 (`self.Tooth_7`))
  (bind _tooth_8 (`self.Tooth_8`))
  (bind _tooth_9 (`self.Tooth_9`))
  (bind _tooth_10 (`self.Tooth_10`))
  (bind _tooth_11 (`self.Tooth_11`))
  (bind _tooth_12 (`self.Tooth_12`))
  (bind _tooth_0 (`self.Tooth_0`))
  (`|ExecutionSequence`
    (:`then_0`
      (if (== (`self.TouchS0`) 1.0)
        (`MeshComponent.SetScalarParameterValueOnMaterials` _tooth_0 "selected" 1.0)
        (else
          (`MeshComponent.SetScalarParameterValueOnMaterials` _tooth_0 "selected" 0.0)))
      (if (== (`self.TouchS1`) 1.0)
        (`MeshComponent.SetScalarParameterValueOnMaterials` _tooth_1 "selected" 1.0)
        (else
          (`MeshComponent.SetScalarParameterValueOnMaterials` _tooth_1 "selected" 0.0)))
      (if (== (`self.TouchS2`) 1.0)
        (`MeshComponent.SetScalarParameterValueOnMaterials` _tooth_2 "selected" 1.0)
        (else
          (`MeshComponent.SetScalarParameterValueOnMaterials` _tooth_2 "selected" 0.0)))
      (if (== (`self.TouchS3`) 1.0)
        (`MeshComponent.SetScalarParameterValueOnMaterials` _tooth_3 "selected" 1.0)
        (else
          (`MeshComponent.SetScalarParameterValueOnMaterials` _tooth_3 "selected" 0.0)))
      (if (== (`self.TouchS4`) 1.0)
        (`MeshComponent.SetScalarParameterValueOnMaterials` _tooth_4 "selected" 1.0)
        (if (== (`self.TouchS5`) 1.0)
          (`MeshComponent.SetScalarParameterValueOnMaterials` _tooth_5 "selected" 1.0)
          (if (== (`self.TouchS6`) 1.0)
            (`MeshComponent.SetScalarParameterValueOnMaterials` _tooth_6 "selected" 1.0)
            (else
              (`MeshComponent.SetScalarParameterValueOnMaterials` _tooth_6 "selected" 0.0)))
          (if (== (`self.TouchS7`) 1.0)
            (`MeshComponent.SetScalarParameterValueOnMaterials` _tooth_7 "selected" 1.0)
            (else
              (`MeshComponent.SetScalarParameterValueOnMaterials` _tooth_7 "selected" 0.0)))
          (if (== (`self.TouchS8`) 1.0)
            (`MeshComponent.SetScalarParameterValueOnMaterials` _tooth_8 "selected" 1.0)
            (else
              (`MeshComponent.SetScalarParameterValueOnMaterials` _tooth_8 "selected" 0.0)))
          (if (== (`self.TouchS9`) 1.0)
            (`MeshComponent.SetScalarParameterValueOnMaterials` _tooth_9 "selected" 1.0)
            (else
              (`MeshComponent.SetScalarParameterValueOnMaterials` _tooth_9 "selected" 0.0)))
          (if (== (`self.TouchS10`) 1.0)
            (`MeshComponent.SetScalarParameterValueOnMaterials` _tooth_10 "selected" 1.0)
            (if (== (`self.TouchS11`) 1.0)
              (`MeshComponent.SetScalarParameterValueOnMaterials` _tooth_11 "selected" 1.0)
              (if (== (`self.TouchS12`) 1.0)
                (`MeshComponent.SetScalarParameterValueOnMaterials` _tooth_12 "selected" 1.0)
                (else
                  (`MeshComponent.SetScalarParameterValueOnMaterials` _tooth_12 "selected" 0.0)))
              (if (== (`self.TouchS13`) 1.0)
                (`MeshComponent.SetScalarParameterValueOnMaterials` _tooth_13 "selected" 1.0)
                (else
                  (`MeshComponent.SetScalarParameterValueOnMaterials` _tooth_13 "selected" 0.0)))
              (else
                (`MeshComponent.SetScalarParameterValueOnMaterials` _tooth_11 "selected" 0.0)))
            (else
              (`MeshComponent.SetScalarParameterValueOnMaterials` _tooth_10 "selected" 0.0)))
          (else
            (`MeshComponent.SetScalarParameterValueOnMaterials` _tooth_5 "selected" 0.0)))
        (else
          (`MeshComponent.SetScalarParameterValueOnMaterials` _tooth_4 "selected" 0.0))))
    (:`then_1`
      (`MeshComponent.SetScalarParameterValueOnMaterials` (`self.force_0`) "selected" (/ (`self.ZoneF0`) 100.0))
      (`MeshComponent.SetScalarParameterValueOnMaterials` (`self.force_1`) "selected" (/ (`self.ZoneF1`) 100.0))
      (`MeshComponent.SetScalarParameterValueOnMaterials` (`self.force_2`) "selected" (/ (`self.ZoneF2`) 100.0))
      (`MeshComponent.SetScalarParameterValueOnMaterials` (`self.force_3`) "selected" (/ (`self.ZoneF3`) 100.0)))))

(fn `UserConstructionScript`)