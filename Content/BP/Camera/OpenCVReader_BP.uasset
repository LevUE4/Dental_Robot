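; OpenCV reader Blueprint that shows a selectable input (webcam, scene capture or player mode) on a raw screen and the OpenCV output texture on a post screen.
; BeginPlay creates the screens' dynamic materials, then opens the camera through MediaPlayer or binds the matching render target.
; In Scene mode, capture runs manually on each OnNextVideoFrame event instead of every frame.
; RenderCamera can draw the raw camera material into the render target.
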(event `self.ReceiveBeginPlay`
  (bind _mediaplayer (`self.MediaPlayer`))
  (`parent.ReceiveBeginPlay`)
  (bind _returnvalue (`PrimitiveComponent.CreateDynamicMaterialInstance` (`self.Screen_Post`) 0 "/Game/BP/Camera/OpenCV_post.OpenCV_Post" "None"))
  (set `self.Material_Post` _returnvalue)
  (bind _returnvalue_2 (`PrimitiveComponent.CreateDynamicMaterialInstance` (`self.Screen_Raw`) 0 "/Game/BP/Camera/OpenCV_Player.OpenCV_Player" "None"))
  (set `self.Material_RenderTarget` _returnvalue_2)
  (switch `EInputMode` (`self.InputMode`)
    (:`Camera`
      (`self.EnableCameraModeBP`)
      (`KismetSystemLibrary.Delay` 0.2)
      (`MediaPlayer.SelectTrack` _mediaplayer "Audio" (`self.VideoTrackID`))
      (`KismetSystemLibrary.Delay` 0.2)
      (`MediaPlayer.Play` _mediaplayer))
    (:`Scene`
      (`self.EnableSceneCapture`))
    (:`Player`
      (`self.EnablePlayerModeBP`)))
  (`KismetSystemLibrary.Delay` 0.2)
  (`MaterialInstanceDynamic.SetTextureParameterValue` (`self.Material_Post`) "OpenCV_Texture" (`self.OpenCV_Texture2D`)))

(event `self.ReceiveTick`
  (params (DeltaSeconds :type "Float (single-precision)"))
  (`parent.ReceiveTick` DeltaSeconds))

(event `self.OnNextVideoFrame`
  (bind _scene_capture (`self.Scene_Capture`))
  (switch `EInputMode` (`self.InputMode`)
    (:`Scene`
      (`/Engine/EditorBlueprintResources/StandardMacros.IsValid` (`self.RenderTarget`)
        (:`Is Valid`
          (`/Engine/EditorBlueprintResources/StandardMacros.IsValid` _scene_capture
            (:`Is Valid`
              (`SceneCaptureComponent2D.CaptureScene` _scene_capture))))))))

(event `self.ValidateCameraID`
  (bind _cameraid (`self.CameraID`))
  (if (< _cameraid 0)
    (set `self.CameraID` 0)
    (else
      (bind _outdevices (`MediaBlueprintFunctionLibrary.EnumerateVideoCaptureDevices` -1))
      (if (< (`KismetArrayLibrary.Array_Length` _outdevices) _cameraid)
        (set `self.CameraID` 0)))))

(event `self.ValidateVideoTrackID`
  (bind _videotrackid (`self.VideoTrackID`))
  (if (< _videotrackid 0)
    (set `self.VideoTrackID` 0)
    (elif (>= _videotrackid (`MediaPlayer.GetNumTracks` (`self.MediaPlayer`) "Video"))
      (set `self.VideoTrackID` 0))))

(fn `EnableCameraModeBP`
  (`self.DisablePlayerMode`)
  (`self.DisableCameraMode`)
  (bind _outdevices (`MediaBlueprintFunctionLibrary.EnumerateVideoCaptureDevices` -1))
  (bind (_output_displayname _output_url) (break `MediaCaptureDevice` (`|GetArrayItem` _outdevices (`self.CameraID`))))
  (`MediaPlayer.OpenUrl` (`self.MediaPlayer`) _output_url)
  (`/Engine/EditorBlueprintResources/StandardMacros.IsValid` (`self.Material_CameraRaw`)
    (:`Is Not Valid`
      (bind _returnvalue (`PrimitiveComponent.CreateDynamicMaterialInstance` (`self.Screen_Raw`) 0 "/Game/BP/Camera/Media_raw.Media_raw" "None"))
      (set `self.Material_CameraRaw` _returnvalue)
      (`MaterialInstanceDynamic.SetTextureParameterValue` (`self.Material_RenderTarget`) "None" (`self.RenderTarget`)))))

(fn `EnablePlayerModeBP`
  (`self.EnablePlayerMode`)
  (`MaterialInstanceDynamic.SetTextureParameterValue` (`self.Material_RenderTarget`) "OpenCV_Texture" (`self.RenderTarget_32Bit`)))

(fn `EnableSceneCapture`
  (bind _rendertarget (`self.RenderTarget`))
  (`self.DisablePlayerMode`)
  (`/Engine/EditorBlueprintResources/StandardMacros.IsValid` (`self.Scene_Capture`)
    (:`Is Valid`
      (`/Engine/EditorBlueprintResources/StandardMacros.IsValid` (`self.RenderTarget`)
        (:`Is Valid`
          (`/Engine/EditorBlueprintResources/StandardMacros.IsValid` (`self.Material_RenderTarget`)
            (:`Is Valid`
              (set `SceneCaptureComponent.bCaptureEveryFrame` false (`self.Scene_Capture`))
              (set `SceneCaptureComponent2D.TextureTarget` _rendertarget (`self.Scene_Capture`))
              (`MaterialInstanceDynamic.SetTextureParameterValue` (`self.Material_RenderTarget`) "OpenCV_Texture" _rendertarget))
            (:`Is Not Valid`
              (bind _returnvalue (`PrimitiveComponent.CreateDynamicMaterialInstance` (`self.Screen_Raw`) 0 "/Game/BP/Camera/OpenCV_Player.OpenCV_Player" "None"))
              (set `self.Material_RenderTarget` _returnvalue))))))))

(fn `RenderCamera`
  (bind _rendertarget (`self.RenderTarget`))
  (bind _material_cameraraw (`self.Material_CameraRaw`))
  (`/Engine/EditorBlueprintResources/StandardMacros.IsValid` _rendertarget
    (:`Is Valid`
      (`/Engine/EditorBlueprintResources/StandardMacros.IsValid` _material_cameraraw
        (:`Is Valid`
          (`KismetRenderingLibrary.DrawMaterialToRenderTarget` _rendertarget _material_cameraraw))))))

(fn `UserConstructionScript`)