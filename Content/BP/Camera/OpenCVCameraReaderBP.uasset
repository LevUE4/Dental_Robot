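; Stereo camera reader actor that fills left and right render targets and shows OpenCV textures on two screens.
; In local camera mode, two scene captures render manually every Tick.
; Otherwise BeginPlay opens two video capture devices through media players with staggered delays, and Tick draws each raw-feed material into its render target.
; Dynamic post materials display the OpenCV output textures, which this graph never writes.
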(event `self.ReceiveBeginPlay`
  (bind _rcamera (`self.RCamera`))
  (bind _rmediaplayer (`self.RMediaPlayer`))
  (bind _lmediaplayer (`self.LMediaPlayer`))
  (bind _lcamera (`self.LCamera`))
  (`parent.ReceiveBeginPlay`)
  (`KismetSystemLibrary.Delay` 0.2)
  (`self.InitializePostTextures`)
  (if (`self.LOCAL_CAMERA_MODE`)
    (set `SceneCaptureComponent.bCaptureEveryFrame` false _rcamera)
    (set `SceneCaptureComponent2D.TextureTarget` (`self.RCameraRenderTarget`) _rcamera)
    (set `SceneCaptureComponent.bCaptureEveryFrame` false _lcamera)
    (set `SceneCaptureComponent2D.TextureTarget` (`self.LCameraRenderTarget`) _lcamera)
    (else
      ;[1 1 1] Left Camera Initializing
      (`self.LCameraInitialize`)
      (bind _outdevices (`MediaBlueprintFunctionLibrary.EnumerateVideoCaptureDevices` -1))
      (bind (_output_displayname _output_url) (break `MediaCaptureDevice` (`|GetArrayItem` _outdevices (`self.LCameraID`))))
      (`MediaPlayer.OpenUrl` (`self.LMediaPlayer`) _output_url)
      (`KismetSystemLibrary.Delay` 1.0)
      (`MediaPlayer.SelectTrack` _lmediaplayer "Video" (`self.LVideoTrackID`))
      (`KismetSystemLibrary.Delay` 1.0)
      (`MediaPlayer.Play` _lmediaplayer)
      ;[1 1 1] Right Camera Initializing
      (`self.RCameraInitialize`)
      (bind _outdevices_2 (`MediaBlueprintFunctionLibrary.EnumerateVideoCaptureDevices` -1))
      (bind (_output_displayname_2 _output_url_2) (break `MediaCaptureDevice` (`|GetArrayItem` _outdevices_2 (`self.RCameraID`))))
      (`MediaPlayer.OpenUrl` (`self.RMediaPlayer`) _output_url_2)
      (`KismetSystemLibrary.Delay` 1.0)
      (`MediaPlayer.SelectTrack` _rmediaplayer "Video" (`self.RVideoTrackID`))
      (`KismetSystemLibrary.Delay` 1.0)
      (`MediaPlayer.Play` _rmediaplayer))))

(event `self.ReceiveTick`
  (params (DeltaSeconds :type "Float (single-precision)"))
  (`parent.ReceiveTick` DeltaSeconds)
  (if (`self.LOCAL_CAMERA_MODE`)
    (`SceneCaptureComponent2D.CaptureScene` (`self.RCamera`))
    (`SceneCaptureComponent2D.CaptureScene` (`self.LCamera`))
    (else
      (`self.RCameraRefresh`)
      (`self.LCameraRefresh`))))

(fn `InitializePostTextures`
  (bind _returnvalue (`PrimitiveComponent.CreateDynamicMaterialInstance` (`self.RScreen`) 0 "/Game/BP/Camera/OpenCV_post.OpenCV_Post" "None"))
  (bind _output_get (set `self.RCameraMaterial` _returnvalue))
  (`MaterialInstanceDynamic.SetTextureParameterValue` _output_get "OpenCV_Texture" (`self.ROpenCV_Texture2D`))
  (bind _returnvalue_2 (`PrimitiveComponent.CreateDynamicMaterialInstance` (`self.LScreen`) 0 "/Game/BP/Camera/OpenCV_post.OpenCV_Post" "None"))
  (bind _output_get_2 (set `self.LCameraMaterial` _returnvalue_2))
  (`MaterialInstanceDynamic.SetTextureParameterValue` _output_get_2 "OpenCV_Texture" (`self.LOpenCV_Texture2D`)))

(fn `LCameraInitialize`
  (bind _lmediatexture (`self.LMediaTexture`))
  (`MediaTexture.SetMediaPlayer` _lmediatexture (`self.LMediaPlayer`))
  (bind _returnvalue (`PrimitiveComponent.CreateDynamicMaterialInstance` (`self.LCamRaw`) 0 "/Game/BP/Camera/OpenCV_post.OpenCV_Post" "None"))
  (`MaterialInstanceDynamic.SetTextureParameterValue` _returnvalue "OpenCV_Texture" _lmediatexture))

(fn `LCameraRefresh`
  (`KismetRenderingLibrary.DrawMaterialToRenderTarget` (`self.LCameraRenderTarget`) (`PrimitiveComponent.GetMaterial` (`self.LCamRaw`) 0)))

(fn `RCameraInitialize`
  (bind _rmediatexture (`self.RMediaTexture`))
  (`MediaTexture.SetMediaPlayer` _rmediatexture (`self.RMediaPlayer`))
  (bind _returnvalue (`PrimitiveComponent.CreateDynamicMaterialInstance` (`self.RCamRaw`) 0 "/Game/BP/Camera/OpenCV_post.OpenCV_Post" "None"))
  (`MaterialInstanceDynamic.SetTextureParameterValue` _returnvalue "OpenCV_Texture" _rmediatexture))

(fn `RCameraRefresh`
  (`KismetRenderingLibrary.DrawMaterialToRenderTarget` (`self.RCameraRenderTarget`) (`PrimitiveComponent.GetMaterial` (`self.RCamRaw`) 0)))

(fn `UserConstructionScript`)