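; RenderCamera_BP shows a live video capture device feed on two screen components, one raw and one post.
; On BeginPlay it creates dynamic materials for both screens and opens the device selected by CameraID in the media player.
; After a short delay it assigns CameraTexture2D to the post material's texture parameter.
; Each Tick draws the raw material into CameraRenderTarget when both are valid.
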(event `self.ReceiveBeginPlay`
  (`parent.ReceiveBeginPlay`)
  (bind _returnvalue (`PrimitiveComponent.CreateDynamicMaterialInstance` (`self.Screen_Raw`) 0 "/Game/BP_/Camera_cv/Camera_Raw.Camera_Raw" "None"))
  (set `self.Camera_MatRaw` _returnvalue)
  (bind _returnvalue_2 (`PrimitiveComponent.CreateDynamicMaterialInstance` (`self.Screen_Post`) 0 "/Game/BP_/Camera_cv/CameraPost.CameraPost" "None"))
  (set `self.Camera_MatPost` _returnvalue_2)
  (bind _outdevices (`MediaBlueprintFunctionLibrary.EnumerateVideoCaptureDevices` -1))
  (`MediaPlayer.OpenUrl` (`self.Camera_MediaPlayer`) (`.Url` (break `MediaCaptureDevice` (`|GetArrayItem` _outdevices (`self.CameraID`)))))
  (`KismetSystemLibrary.Delay` 0.2)
  (`MaterialInstanceDynamic.SetTextureParameterValue` (`self.Camera_MatPost`) "Texture" (`self.Camera_Texture2D`)))

(event `self.ReceiveTick`
  (params (DeltaSeconds :type "Float (single-precision)"))
  (bind _camera_rendertarget (`self.Camera_RenderTarget`))
  (bind _camera_matraw (`self.Camera_MatRaw`))
  (`parent.ReceiveTick` DeltaSeconds)
  (`/Engine/EditorBlueprintResources/StandardMacros.IsValid` _camera_rendertarget
    (:`Is Valid`
      (`/Engine/EditorBlueprintResources/StandardMacros.IsValid` _camera_matraw
        (:`Is Valid`
          (`KismetRenderingLibrary.DrawMaterialToRenderTarget` _camera_rendertarget _camera_matraw))))))

(fn `UserConstructionScript`)